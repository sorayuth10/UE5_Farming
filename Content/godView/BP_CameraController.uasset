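; God-view camera controller that pans by touch drag and zooms a spring arm, with mouse cursor and touch events enabled.
; Tick turns first-touch screen movement into an axis-swapped world offset on the actor.
; ZoomCamera sets arm length from GetTouchDistance (two-finger gap, or cursor position on Windows), scaled by zoom range over viewport diagonal.
; Zoom looks unfinished: the event's starting-value captures never run, and the Pinch Camera Zoom graph's calculation is unused.
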(event `self.ReceiveBeginPlay`
  (bind _returnvalue (`GameplayStatics.GetPlayerController` 0))
  (set `PlayerController.bShowMouseCursor` true _returnvalue)
  (set `PlayerController.bEnableTouchEvents` true _returnvalue))

(event `InputAction|DragCamera`
  (params (Key :type "Key Structure"))
  (bind (_locationx _locationy) (`PlayerController.GetInputTouchState` (`GameplayStatics.GetPlayerController` 0) "Touch1"))
  (:`Pressed`
    (set `self.Previous Touch Location` (`KismetMathLibrary.MakeVector2D` _locationx _locationy))))

(event `self.ReceiveTick`
  (params (DeltaSeconds :type "Float (single-precision)"))
  (bind (_locationx _locationy _biscurrentlypressed) (`PlayerController.GetInputTouchState` (`GameplayStatics.GetPlayerController` 0) "Touch1"))
  (bind (_returnvalue_x _returnvalue_y) (`KismetMathLibrary.BreakVector2D` (- (`self.New Touch Location`) (`self.Previous Touch Location`))))
  (if _biscurrentlypressed
    (set `self.New Touch Location` (`KismetMathLibrary.MakeVector2D` _locationx _locationy))
    (`self.K2_AddActorWorldOffset` (`KismetMathLibrary.MakeVector` _returnvalue_y (* _returnvalue_x -1.0)))
    (set `self.Previous Touch Location` (`self.New Touch Location`))))

(event `EnhancedInput|/Game/TopDown/Input/ZoomCamera`
  (params (ActionValue :type Boolean) (ElapsedSeconds :type "Float (double-precision)") (TriggeredSeconds :type "Float (double-precision)") (InputAction :type "InputAction Object Reference" :default "/Game/TopDown/Input/ZoomCamera.ZoomCamera"))
  (:`Triggered`
    (set `SpringArmComponent.TargetArmLength` (* (- (`self.Get Touch Distance`) (`|TemporaryVariable`)) (/ (- (`self.Max Zoom Distance`) (`self.Min Zoom Distance`)) (`KismetMathLibrary.VSize2D` (`WidgetLayoutLibrary.GetViewportSize`)))) (`self.SpringArm`))))

(fn `Get Touch Distance`
  (returns (`Touch distance` :type "Float (double-precision)"))
  (bind _returnvalue (`GameplayStatics.GetPlayerController` 0))
  (bind (_locationx _locationy) (`PlayerController.GetInputTouchState` _returnvalue "Touch2"))
  (bind (_locationx_2 _locationy_2) (`PlayerController.GetMousePosition` _returnvalue))
  (bind (_locationx_3 _locationy_3) (`PlayerController.GetInputTouchState` _returnvalue "Touch1"))
  (return (`KismetMathLibrary.VSize2D` (select `bool` (`KismetStringLibrary.EqualEqual_StrStr` (`GameplayStatics.GetPlatformName`) "Windows") :`false` (- (`KismetMathLibrary.MakeVector2D` _locationx_3 _locationy_3) (`KismetMathLibrary.MakeVector2D` _locationx _locationy)) :`true` (`KismetMathLibrary.MakeVector2D` _locationx_2 _locationy_2)))))

(fn `UserConstructionScript`)